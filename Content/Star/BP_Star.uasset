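; Procedurally generated star actor that picks a spectral class and luminosity class, Hertzsprung-Russell style, and spawns a planet.
; Construction rolls class, temperature and mass from a seed stream, though the luminosity value itself is unseeded.
; StarRuleSystem turns these into sphere scale, debug labels, dynamic material colour, glow and movement, and light settings, rerunning at BeginPlay.
; PlanetBuilder then places one BP_Planet and sets a camera location, both scaled by mass times temperature.
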(event Custom|Planet%20Builder
  (bind _sphere (Variables|Default|GetSphere))
  (bind _setmass (Variables|Default|GetSetMass))
  (bind _settemp (Variables|Default|GetSetTemp))
  (bind _returnvalue (Transformation|GetWorldLocation _sphere))
  (bind _returnvalue_2 (* _setmass _settemp))
  (bind _returnvalue_3 (* _returnvalue_2 9e+02))
  (bind _returnvalue_4 (* _returnvalue_2 3e+02))
  (bind _returnvalue_5 (Math|Vector|MakeVector 0.0 0.0 _returnvalue_3))
  (bind _returnvalue_6 (Math|Vector|MakeVector _returnvalue_4 _returnvalue_4 _returnvalue_4))
  (Development|PrintString (Utilities|String|Append "Distance" (Utilities|String|ToString(Float) _returnvalue_2)))
  (Variables|Default|SetSystemLen _returnvalue_4)
  (Collision|MultiLineTraceByChannel _returnvalue _returnvalue_6 "TraceTypeQuery1" false 0 "Persistent")
  (Game|SpawnActorfromClass "/Game/Planets/BP_Planet.BP_Planet_C" (Math|Conversions|ToTransform(Vector) _returnvalue_6) "Undefined" 0 0)
  (Collision|MultiLineTraceByChannel _returnvalue _returnvalue_5 "TraceTypeQuery1" false 0 "ForOneFrame")
  (Variables|Default|SetCameraLocation _returnvalue_5))

(event EventBeginPlay
  (CallFunction|StarRuleSystem (Variables|Default|GetStar_Holder) (Variables|Default|GetStarLuminHolder))
  (CallFunction|PlanetBuilder))

(event Collision|EventActorBeginOverlap
  (params (OtherActor :type Actor%20Object%20Reference)))

(event EventTick
  (params (DeltaSeconds :type Float%20%28single-precision%29)))

(fn ConstructionScript
  (bind _seed (Variables|Default|GetSeed))
  (bind _startype (Variables|Default|GetStarType))
  (bind (_typeofsun _luminous) (Utilities|Struct|BreakStruct_StarData _startype))
  (bind _returnvalue (Math|Random|RandomIntegerinRangefromStream 0 7 _seed))
  ;[1 1 1] Seed Generation + Setting the Lumen and Star Type
  (bind _output_get (LocalVariables|SetSeedGenerator _returnvalue))
  (Development|PrintString (Utilities|String|Append "SEED GEN :: " (Utilities|String|ToString(Integer) _output_get)))
  (bind _output_get_2 (Variables|Default|SetStar_Holder (Utilities|Array|Get(acopy) _typeofsun _returnvalue)))
  (bind _output_get_3 (Variables|Default|SetStarLuminHolder (Utilities|Array|Get(acopy) _luminous (Math|Random|RandomIntegerinRangefromStream 0 9 _seed))))
  (Development|PrintString (Utilities|String|Append "SUN CLASS :: " (Utilities|String|EnumtoString _output_get_2) "Lumin :::" (Utilities|String|EnumtoString _output_get_3)))
  (CallFunction|SetTempandMass (Math|Conversions|ToInteger(Byte) (Math|Byte|MakeLiteralByte _output_get_2)))
  (CallFunction|StarRuleSystem (Variables|Default|GetStar_Holder) (Variables|Default|GetStarLuminHolder)))

(fn SetTempandMass
  (params (SunTypeIndex :type Integer))
  (bind _starmetadata (Variables|Default|GetStarMetaData))
  (bind (_mintemp _maxtemp _minmass _maxmass) (Utilities|Struct|BreakE_StarData _starmetadata))
  (bind _output_get (Variables|Default|SetMinTemp (Utilities|Array|Get(acopy) _mintemp SunTypeIndex)))
  (bind _output_get_2 (Variables|Default|SetMaxTemp (Utilities|Array|Get(acopy) _maxtemp SunTypeIndex)))
  (bind _output_get_3 (Variables|Default|SetMinMass (Utilities|Array|Get(acopy) _minmass SunTypeIndex)))
  (bind _output_get_4 (Variables|Default|SetMaxMass (Utilities|Array|Get(acopy) _maxmass SunTypeIndex)))
  (Variables|Default|SetSetTemp (Math|Random|RandomFloatinRangefromStream _output_get _output_get_2 (Variables|Default|GetSeed)))
  (Variables|Default|SetSetMass (Math|Random|RandomFloatinRangefromStream _output_get_3 _output_get_4 (Variables|Default|GetSeed))))

(fn StarRuleSystem
  (params (Star :type E_StarTypes%20Enum :default "NewEnumerator0") (Luminous :type E_luminous%20Enum :default "NewEnumerator0"))
  (bind _setmass (Variables|Default|GetSetMass))
  ;[1 1 1] Resizes Star
  (Transformation|SetWorldScale3D (Variables|Default|GetSphere) (* "1.000000,1.000000,1.000000" _setmass))
  ;[1 0.6129 0] Debug Only
  (Rendering|Components|TextRender|SetText (Variables|Default|GetClass) (Utilities|Text|FormatText "{class}" (Utilities|String|EnumtoString Star)))
  (Rendering|Components|TextRender|SetText (Variables|Default|GetLuminous) (Utilities|Text|FormatText "Luminous: {lumin}" (Utilities|String|EnumtoString Luminous)))
  ;[1 1 1] Sets Mass
  (Class|PrimitiveComponent|SetMassScale (Variables|Default|GetSphere) "None" _setmass)
  ;[1 1 1] Hertzsprung-Russell
  (bind _output_value (CallFunction|StarLuminous Luminous))
  (bind _starcolour (CallFunction|StarColour Star Luminous _output_value))
  (bind _emissiveout (CallFunction|SetEmissive))
  ;[1 1 1] Material Generation
  (bind _returnvalue (CallFunction|StarMovement))
  (CallFunction|StarMaterial _starcolour _emissiveout _output_value _returnvalue)
  ;[1 1 1] Lights
  (Rendering|Lighting|SetAttenuationRadius (Variables|Default|GetPointLight) (* (Variables|Default|GetSetTemp) 5e+02))
  (Rendering|Components|Light|SetLightColor (Variables|Default|GetPointLight) _starcolour true))

(fn StarMaterial
  (params (Star%20Class%20Colour :type Linear%20Color%20Structure) (StarEmissive :type Float%20%28single-precision%29) (StarLumenious :type Float%20%28single-precision%29) (StarMovement :type Float%20%28single-precision%29))
  (bind _returnvalue (Rendering|Material|CreateDynamicMaterialInstance (Variables|Default|GetSphere) 0 "/Game/Materials/M_Star.M_Star" "None" :!class /Script/Engine.PrimitiveComponent))
  (Rendering|Material|SetVectorParameterValue _returnvalue "StarColourParam" Star%20Class%20Colour :!class /Script/Engine.MaterialInstanceDynamic)
  (Rendering|Material|SetScalarParameterValue _returnvalue "StarEmissiveControlParam" StarEmissive :!class /Script/Engine.MaterialInstanceDynamic) ; Deals with Light being Drawn 0.1 - 0.0000001
  (Rendering|Material|SetScalarParameterValue _returnvalue "StarLumeniousParam" StarLumenious :!class /Script/Engine.MaterialInstanceDynamic)
  (Rendering|Material|SetScalarParameterValue _returnvalue "MassMovementParam" StarMovement :!class /Script/Engine.MaterialInstanceDynamic))

(fn StarColour
  (params (StarType :type E_StarTypes%20Enum :default "NewEnumerator0") (StarLuminous :type E_luminous%20Enum :default "NewEnumerator0") (Determinor :type Float%20%28double-precision%29))
  (bind _returnvalue (/ Determinor 1e+02))
  (bind _returnvalue_2 (/ Determinor 1e+02))
  (switch Utilities|FlowControl|Switch|SwitchonE_luminous StarLuminous
    (:NewEnumerator0
      _)
    (:NewEnumerator1
      _)
    (:NewEnumerator2
      _)
    (:NewEnumerator3
      _)
    (:NewEnumerator4
      _)
    (:NewEnumerator5
      _)
    (:NewEnumerator6
      _)
    (:NewEnumerator7
      _)
    (:NewEnumerator8
      (bind _output_get (LocalVariables|SetColourVector "(R=0.000000,G=0.081324,B=0.468750,A=1.000000)"))
      (return (+ _output_get _returnvalue)))
    (:NewEnumerator9
      (bind _output_get_2 (LocalVariables|SetColourVector "(R=0.155165,G=0.502282,B=0.677083,A=1.000000)"))
      (return (+ _output_get_2 _returnvalue))))
  (switch Utilities|FlowControl|Switch|SwitchonE_StarTypes StarType
    (:NewEnumerator0
      (bind _output_get_3 (LocalVariables|SetColourVector "(R=0.000000,G=0.021972,B=0.343750,A=1.000000)"))
      (return (+ _output_get_3 _returnvalue_2)))
    (:NewEnumerator1
      (bind _output_get_4 (LocalVariables|SetColourVector "(R=0.213542,G=0.503548,B=1.000000,A=1.000000)"))
      (return (+ _output_get_4 _returnvalue_2)))
    (:NewEnumerator2
      (bind _output_get_5 (LocalVariables|SetColourVector "(R=0.968750,G=1.000000,B=0.937500,A=1.000000)"))
      (return (+ _output_get_5 _returnvalue_2)))
    (:NewEnumerator3
      (bind _output_get_6 (LocalVariables|SetColourVector "(R=1.000000,G=0.947682,B=0.508316,A=1.000000)"))
      (return (+ _output_get_6 _returnvalue_2)))
    (:NewEnumerator4
      (bind _output_get_7 (LocalVariables|SetColourVector "(R=1.000000,G=0.763262,B=0.000000,A=1.000000)"))
      (return (+ _output_get_7 _returnvalue_2)))
    (:NewEnumerator5
      (bind _output_get_8 (LocalVariables|SetColourVector "(R=0.916667,G=0.434080,B=0.006739,A=1.000000)"))
      (return (+ _output_get_8 _returnvalue_2)))
    (:NewEnumerator6
      (bind _output_get_9 (LocalVariables|SetColourVector "(R=0.906250,G=0.228759,B=0.018880,A=1.000000)"))
      (return (+ _output_get_9 _returnvalue_2)))))

(fn StarLuminous
  (params (Star%20Luminous :type E_luminous%20Enum :default "NewEnumerator0"))
  (switch Utilities|FlowControl|Switch|SwitchonE_luminous Star%20Luminous ; 1 = low 100 = high
    (:NewEnumerator0
      ;[1 1 1] 0 or La
      (bind _output_get (LocalVariables|SetLumiousVal (Math|Random|RandomFloatinRange 9e+01 1e+02)))
      (return _output_get))
    (:NewEnumerator1
      ;[1 1 1] La
      (bind _output_get_2 (LocalVariables|SetLumiousVal (Math|Random|RandomFloatinRange 7e+01 9e+01)))
      (return _output_get_2))
    (:NewEnumerator2
      ;[1 1 1] Lab
      (bind _output_get_3 (LocalVariables|SetLumiousVal (Math|Random|RandomFloatinRange 5e+01 7e+01)))
      (return _output_get_3))
    (:NewEnumerator3
      ;[1 1 1] Lb
      (bind _output_get_4 (LocalVariables|SetLumiousVal (Math|Random|RandomFloatinRange 4e+01 6e+01)))
      (return _output_get_4))
    (:NewEnumerator4
      ;[1 1 1] ll
      (bind _output_get_5 (LocalVariables|SetLumiousVal (Math|Random|RandomFloatinRange 3e+01 5e+01)))
      (return _output_get_5))
    (:NewEnumerator5
      ;[1 1 1] lll
      (bind _output_get_6 (LocalVariables|SetLumiousVal (Math|Random|RandomFloatinRange 2e+01 4e+01)))
      (return _output_get_6))
    (:NewEnumerator6
      ;[1 1 1] Iv
      (bind _output_get_7 (LocalVariables|SetLumiousVal (Math|Random|RandomFloatinRange 1e+01 2e+01)))
      (return _output_get_7))
    (:NewEnumerator7
      ;[1 1 1] V
      (bind _output_get_8 (LocalVariables|SetLumiousVal (Math|Random|RandomFloatinRange 5.0 1e+01)))
      (return _output_get_8))
    (:NewEnumerator8
      ;[1 1 1] Sd or VI
      (bind _output_get_9 (LocalVariables|SetLumiousVal (Math|Random|RandomFloatinRange 3.0 5.0)))
      (return _output_get_9))
    (:NewEnumerator9
      ;[1 1 1] D or VII
      (bind _output_get_10 (LocalVariables|SetLumiousVal (Math|Random|RandomFloatinRange 0.1 3.0)))
      (return _output_get_10))))

(fn SetEmissive
  (switch Utilities|FlowControl|Switch|SwitchonE_luminous (Variables|Default|GetStarLuminHolder)
    (:NewEnumerator0
      ;[1 1 1] 0 or LA
      (bind _output_get (LocalVariables|SetRandomEmissive (Math|Random|RandomFloatinRangefromStream 1e-06 0.0001 (Variables|Default|GetSeed))))
      (return _output_get))
    (:NewEnumerator1
      ;[1 1 1] LA
      (bind _output_get_2 (LocalVariables|SetRandomEmissive (Math|Random|RandomFloatinRangefromStream 1e-06 0.001 (Variables|Default|GetSeed))))
      (return _output_get_2))
    (:NewEnumerator2
      ;[1 1 1] lab
      (bind _output_get_3 (LocalVariables|SetRandomEmissive (Math|Random|RandomFloatinRangefromStream 1e-05 0.01 (Variables|Default|GetSeed))))
      (return _output_get_3))
    (:NewEnumerator3
      ;[1 1 1] lb
      (bind _output_get_4 (LocalVariables|SetRandomEmissive (Math|Random|RandomFloatinRangefromStream 0.0001 0.01 (Variables|Default|GetSeed))))
      (return _output_get_4))
    (:NewEnumerator4
      ;[1 1 1] ll
      (bind _output_get_5 (LocalVariables|SetRandomEmissive (Math|Random|RandomFloatinRangefromStream 0.0001 0.1 (Variables|Default|GetSeed))))
      (return _output_get_5))
    (:NewEnumerator5
      ;[1 1 1] lll
      (bind _output_get_6 (LocalVariables|SetRandomEmissive (Math|Random|RandomFloatinRangefromStream 0.001 0.1 (Variables|Default|GetSeed))))
      (return _output_get_6))
    (:NewEnumerator6
      ;[1 1 1] IV
      (bind _output_get_7 (LocalVariables|SetRandomEmissive (Math|Random|RandomFloatinRangefromStream 0.01 0.1 (Variables|Default|GetSeed))))
      (return _output_get_7))
    (:NewEnumerator7
      ;[1 1 1] V
      (bind _output_get_8 (LocalVariables|SetRandomEmissive (Math|Random|RandomFloatinRangefromStream 0.01 0.1 (Variables|Default|GetSeed))))
      (return _output_get_8))
    (:NewEnumerator8
      ;[1 1 1] Sd or Vi
      (bind _output_get_9 (LocalVariables|SetRandomEmissive (Math|Random|RandomFloatinRangefromStream 1e-06 0.01 (Variables|Default|GetSeed))))
      (return _output_get_9))
    (:NewEnumerator9
      ;[1 1 1] D or Vii
      (bind _output_get_10 (LocalVariables|SetRandomEmissive (Math|Random|RandomFloatinRangefromStream 1e-06 0.1 (Variables|Default|GetSeed))))
      (return _output_get_10))))

(fn StarMovement
  (return (Math|Float|Clamp(Float) (* (/ (Math|Random|RandomFloatinRangefromStream 0.0001 (Variables|Default|GetSetMass) (Variables|Default|GetSeed)) (Math|Random|RandomFloatinRangefromStream 0.0001 (Variables|Default|GetSetTemp) (Variables|Default|GetSeed))) 2.0) 0.1)))